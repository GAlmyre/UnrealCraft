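; BP_ControllerTest is a controller that adds RTS-style screen-edge scrolling for a controlled CameraPawn.
; Each Tick it reads the viewport size and mouse position, then casts and stores the controlled pawn.
; When the cursor sits within a thin band at a screen edge, it calls the pawn's MoveRight or MoveForward with a fixed signed amount, not scaled by delta time.
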(event `self.ReceiveTick`
  (params (DeltaSeconds :type "Float (single-precision)"))
  (bind (_locationx _locationy) (`self.GetMousePosition`))
  (bind _mousex (`self.MouseX`))
  (bind _viewportsize_x (`KismetMathLibrary.BreakVector2D` (`self.ViewportSize`)))
  (bind (_viewportsize_x_2 _viewportsize_y) (`KismetMathLibrary.BreakVector2D` (`self.ViewportSize`)))
  (bind _mousey (`self.MouseY`))
  (bind _mousey_2 (`self.MouseY`))
  (bind _mousex_2 (`self.MouseX`))
  (set `self.ViewportSize` (`WidgetLayoutLibrary.GetViewportSize`))
  (set `self.MouseX` _locationx)
  (set `self.MouseY` _locationy)
  (bind _ascamera_pawn (cast `CameraPawn` (`self.K2_GetPawn`)))
  (set `self.PawnVar` _ascamera_pawn)
  (if (and (>= _mousex_2 0.0) (<= _mousex_2 2.0))
    (`DefaultPawn.MoveRight` (`self.PawnVar`) -10.0)
    (elif (and (>= _mousex (- _viewportsize_x 2.0)) (<= _mousex _viewportsize_x))
      (`DefaultPawn.MoveRight` (`self.PawnVar`) 10.0)))
  (if (and (>= _mousey 0.0) (<= _mousey 2.0))
    (`DefaultPawn.MoveForward` (`self.PawnVar`) 10.0)
    (elif (and (>= _mousey_2 (- _viewportsize_y 2.0)) (<= _mousey_2 _viewportsize_y))
      (`DefaultPawn.MoveForward` (`self.PawnVar`) -10.0))))

(fn `UserConstructionScript`)